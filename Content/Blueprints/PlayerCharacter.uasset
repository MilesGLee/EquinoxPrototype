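; Third-person wraith player character that can sink into shadow with Left Shift and glide along surfaces.
; Tick drives camera, camera-relative movement, rotation smoothing, animation and a shadow test that traces to every PointLight, blocking dives when visible within a multiple of its source radius.
; While diving in Flying mode, down and forward traces supply a surface normal to stick and align to; light or lost ground ends the dive.
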(event Custom|RotateCameraArm
  (bind _cameraspringarm (Variables|Default|GetCameraSpringArm))
  (bind _relativerotation (Variables|/Script/Engine.SceneComponent|GetRelativeRotation _cameraspringarm))
  ;[1 1 1] Rotate Camera Arm
  (Transformation|AddRelativeRotation (Variables|Default|GetCameraSpringArm) (Math|Rotator|MakeRotator 0.0 (Variables|Default|GetVerticalMouseInput) (Variables|Default|GetHorizontalMouseInput)) false false)
  (Transformation|SetRelativeRotation _cameraspringarm (Math|Rotator|MakeRotator 0.0 (Math|Float|Clamp(Float) (.pitch _relativerotation) -7e+01 7e+01) (.yaw _relativerotation)) false false))

(event Custom|MoveCharacter
  ;[1 1 1] Move Character
  (Pawn|Input|AddMovementInput (Math|Vector|Normalize (* (Math|Vector|GetForwardVector (Variables|Default|GetPlayerCamera)) (Variables|Default|GetVerticalKeyInput))) 1e+01 false)
  (Pawn|Input|AddMovementInput (Math|Vector|Normalize (* (Math|Vector|GetRightVector (Variables|Default|GetPlayerCamera)) (Variables|Default|GetHorizontalKeyInput))) 1e+01 false))

(event Custom|Rotate%20Orientation
  ;[1 1 1] Rotate Orientation
  (Transformation|SetRelativeRotation (Variables|Default|GetOrientation) (Math|Rotator|Lerp(Rotator) (Variables|/Script/Engine.SceneComponent|GetRelativeRotation (Variables|Default|GetOrientation)) (Math|Rotator|MakeRotator 0.0 0.0 (.yaw (Variables|/Script/Engine.SceneComponent|GetRelativeRotation (Variables|Default|GetCameraSpringArm)))) 0.05 true) false false))

(event Custom|OnDiveTick
  (bind _orientation (Variables|Default|GetOrientation))
  (bind _charactermovement (Variables|Character|GetCharacterMovement))
  (bind _orientation_2 (Variables|Default|GetOrientation))
  (bind _orientation_3 (Variables|Default|GetOrientation))
  (bind _returnvalue (Transformation|GetWorldLocation _orientation))
  (bind _returnvalue_2 (Transformation|GetWorldLocation _orientation_2))
  (bind _returnvalue_3 (Math|Vector|GetUpVector _orientation_3))
  ;[1 1 1] On Dive Tick
  (if (Variables|Default|GetCanDive)
    (bind (_outhit _returnvalue_4) (Collision|LineTraceByChannel _returnvalue (+ _returnvalue (* (Math|Vector|GetUpVector _orientation) -1e+02)) "TraceTypeQuery1" false 0 "ForDuration"))
    (if _returnvalue_4
      (bind (_outhit_2 _returnvalue_5) (Collision|LineTraceByChannel _returnvalue_2 (+ _returnvalue_2 (* (Math|Vector|GetForwardVector _orientation_2) 1e+02)) "TraceTypeQuery1" false 0 "ForDuration"))
      (if _returnvalue_5
        (Variables|Default|SetNormalVector (.normal _outhit_2))
        (Pawn|Input|AddMovementInput (* (Variables|Default|GetNormalVector) -1.0) 1e+01 false :!label _label)
        (if (not (and (== (Variables|Default|GetVerticalKeyInput) 0.0) (== (Variables|Default|GetHorizontalKeyInput) 0.0)))
          _
          (else
            (Variables|/Script/Engine.MovementComponent|SetVelocity _charactermovement (* (Variables|/Script/Engine.MovementComponent|GetVelocity _charactermovement) 0.9))))
        (Transformation|SetWorldRotation (Variables|Character|GetMesh) (Math|Rotator|Lerp(Rotator) (Transformation|GetWorldRotation (Variables|Default|GetOrientation)) (Math|Rotator|MakeRotfromZX (Variables|Default|GetNormalVector) (Math|Vector|RotateVectorAroundAxis (Math|Vector|GetForwardVector _orientation_3) (* (Class|KismetMathLibrary|DegAcos (Math|Vector|DotProduct (Variables|Default|GetNormalVector) _returnvalue_3)) -1.0) (Math|Vector|Normalize (Math|Vector|CrossProduct (Variables|Default|GetNormalVector) _returnvalue_3)))) 0.07 true) false false)
        (Transformation|SetWorldRotation (Variables|Default|GetOrientation) (Math|Rotator|Lerp(Rotator) (Transformation|GetWorldRotation (Variables|Default|GetOrientation)) (Math|Rotator|MakeRotfromZX (Variables|Default|GetNormalVector) (Math|Vector|RotateVectorAroundAxis (Math|Vector|GetForwardVector _orientation_3) (* (Class|KismetMathLibrary|DegAcos (Math|Vector|DotProduct (Variables|Default|GetNormalVector) _returnvalue_3)) -1.0) (Math|Vector|Normalize (Math|Vector|CrossProduct (Variables|Default|GetNormalVector) _returnvalue_3)))) 0.07 true) false false)
        (elif _returnvalue_4
          (Variables|Default|SetNormalVector (.normal _outhit))
          (goto _label)
          (else
            (CallFunction|OnDive))))
      (else
        (CallFunction|OnDive)))
    (else
      (CallFunction|OnDive))))

(event Custom|OnDive
  (bind _charactermovement (Variables|Character|GetCharacterMovement))
  ;[1 1 1] On Dive Event
  (if (not (Variables|Default|GetIsDiving))
    (Components|Animation|PlayAnimation (Variables|Character|GetMesh) "/Game/Animations/AS_WraithPrototype_Sink_Anim.AS_WraithPrototype_Sink_Anim" false)
    (Utilities|FlowControl|Delay 1.0)
    (Pawn|Components|CharacterMovement|SetMovementMode _charactermovement "MOVE_Flying" 0)
    (else
      (Pawn|Components|CharacterMovement|SetMovementMode _charactermovement "MOVE_Walking" 0)
      (Variables|Default|SetGravityDirection "0,0.000000,-1.000000")
      (Components|Animation|PlayAnimation (Variables|Character|GetMesh) "/Game/Animations/AS_WraithPrototype_Idle_Anim.AS_WraithPrototype_Idle_Anim" false)))
  (Variables|Default|SetIsDiving (not (Variables|Default|GetIsDiving))))

(event Custom|RotateMesh
  ;[1 1 1] Rotate Mesh
  (Transformation|SetRelativeRotation (Variables|Character|GetMesh) (Math|Rotator|Lerp(Rotator) (Variables|/Script/Engine.SceneComponent|GetRelativeRotation (Variables|Character|GetMesh)) (Math|Rotator|MakeRotator 0.0 0.0 (+ -9e+01 (.yaw (Variables|/Script/Engine.SceneComponent|GetRelativeRotation (Variables|Default|GetCameraSpringArm))))) 0.05 true) false false))

(event Custom|AnimateMesh
  ;[1 1 1] Animate Mesh
  (if (not (and (== (Variables|Default|GetVerticalKeyInput) 0.0) (== (Variables|Default|GetHorizontalKeyInput) 0.0)))
    (if (Variables|Default|GetIsDiving)
      (Utilities|FlowControl|DoOnce false :!label _label
        (:Completed
          (Components|Animation|PlayAnimation (Variables|Character|GetMesh) "/Game/Animations/AS_WraithPrototype_SinkRun_Anim.AS_WraithPrototype_SinkRun_Anim" true)
          (goto _label_3 Reset)))
      (else
        (Utilities|FlowControl|DoOnce false :!label _label_2
          (:Completed
            (Components|Animation|PlayAnimation (Variables|Character|GetMesh) "/Game/Animations/AS_WraithPrototype_Run_Anim.AS_WraithPrototype_Run_Anim" true)
            (goto _label_4 Reset)))))
    (elif (Variables|Default|GetIsDiving)
      (Utilities|FlowControl|DoOnce false :!label _label_3
        (:Completed
          (Components|Animation|PlayAnimation (Variables|Character|GetMesh) "/Game/Animations/AS_WraithPrototype_SinkIdle_Anim.AS_WraithPrototype_SinkIdle_Anim" true)
          (goto _label Reset)))
      (else
        (Utilities|FlowControl|DoOnce false :!label _label_4
          (:Completed
            (Components|Animation|PlayAnimation (Variables|Character|GetMesh) "/Game/Animations/AS_WraithPrototype_Idle_Anim.AS_WraithPrototype_Idle_Anim" true)
            (goto _label_2 Reset)))))))

(event Custom|CheckIfCanDive
  ;[1 1 1] Check if can dive
  (Variables|Default|SetCanDive true)
  (bind _outactors (Actor|GetAllActorsOfClass "/Script/Engine.PointLight"))
  (bind _array_element (Utilities|Array|ForEachLoopwithBreak _outactors :!label _label)
    (:LoopBody
      (Variables|Default|SetCurrentActor _array_element)
      (bind _returnvalue (Collision|LineTraceByChannel (Transformation|GetWorldLocation (Variables|Default|GetOrientation)) (Transformation|GetActorLocation (Variables|Default|GetCurrentActor)) "TraceTypeQuery1" false 0 "None"))
      (if (not _returnvalue)
        (if (> (Math|Vector|VectorLength (- (Transformation|GetWorldLocation (Variables|Default|GetOrientation)) (Transformation|GetActorLocation (Variables|Default|GetCurrentActor)))) (* (Variables|/Script/Engine.PointLightComponent|GetSourceRadius (Actor|GetComponentbyClass (Variables|Default|GetCurrentActor) "/Script/Engine.PointLightComponent")) 3.0))
          (Variables|Default|SetCanDive true)
          (else
            (Variables|Default|SetCanDive false)
            (goto _label Break)))
        (else
          (Variables|Default|SetCanDive true))))))

(event EventTick
  (params (DeltaSeconds :type Float%20%28single-precision%29))
  (CallFunction|RotateCameraArm)
  (CallFunction|MoveCharacter)
  (CallFunction|RotateMesh)
  (CallFunction|RotateOrientation)
  (CallFunction|AnimateMesh)
  (CallFunction|CheckifCanDive)
  (if (Variables|Default|GetIsDiving)
    (CallFunction|OnDiveTick)))

(event Input|AxisEvents|InputAxisHorizontalKeyInput
  (params (AxisValue :type Float%20%28single-precision%29))
  (Variables|Default|SetHorizontalKeyInput AxisValue))

(event Input|AxisEvents|InputAxisVerticalKeyInput
  (params (AxisValue :type Float%20%28single-precision%29))
  (Variables|Default|SetVerticalKeyInput AxisValue))

(event Input|AxisEvents|InputAxisHorizontalMouseInput
  (params (AxisValue :type Float%20%28single-precision%29))
  (Variables|Default|SetHorizontalMouseInput AxisValue))

(event Input|AxisEvents|InputAxisVerticalMouseInput
  (params (AxisValue :type Float%20%28single-precision%29))
  (Variables|Default|SetVerticalMouseInput AxisValue))

(event Input|KeyboardEvents|LeftShift
  (params (Key :type Key%20Structure :default "None"))
  (:Pressed
    (CallFunction|CheckifCanDive)
    (if (Variables|Default|GetCanDive)
      (CallFunction|OnDive))))

(fn ConstructionScript)